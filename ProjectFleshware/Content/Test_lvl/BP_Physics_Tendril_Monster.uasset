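; Wrapper actor pairing a physics-simulated tendril mesh with a child-actor tendril monster that ambushes the VR player once.
; On BeginPlay it enables mesh physics, caches the monster and snaps the trigger sphere to its pelvis socket.
; The first player overlap triggers the monster's GroundSmashAttack, then a delayed CheckIfDead destroys the actor.
; CheckIfDead only validates the child actor class, with no health or death test.
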(event OnComponentBeginOverlap(Sphere)
  (params (OverlappedComponent :type Primitive%20Component%20Object%20Reference) (OtherActor :type Actor%20Object%20Reference) (OtherComp :type Primitive%20Component%20Object%20Reference) (OtherBodyIndex :type Integer) (bFromSweep :type Boolean) (SweepResult :type Hit%20Result%20Structure%20%28by%20ref%29))
  (bind _asbp_rais_vr_character (Utilities|Casting|CastToBP_RAIS_VR_Character OtherActor))
  (Utilities|IsValid _asbp_rais_vr_character
    (:Is%20Valid
      (Utilities|FlowControl|DoOnce false
        (:Completed
          (Default|GroundSmashAttack (Variables|Default|GetTendrilMonster_Ref) _asbp_rais_vr_character)
          (Utilities|FlowControl|Delay 4.0)
          (CallFunction|CheckifDead))))))

(event Custom|Check%20If%20Dead
  (if (Utilities|IsValidClass (Variables|/Script/Engine.ChildActorComponent|GetChildActorClass (Variables|Default|GetEnemy)))
    (Utilities|FlowControl|Delay 3.0)
    (Actor|DestroyActor)))

(event EventBeginPlay
  (Physics|SetSimulatePhysics (Variables|Default|GetTendril_Mesh) true)
  (bind _ascbp_enemy__tendril_monst (Utilities|Casting|CastToCBP-Enemy-Tendril_Monst (Variables|/Script/Engine.ChildActorComponent|GetChildActor (Variables|Default|GetEnemy))))
  (Variables|Default|SetTendrilMonster_Ref _ascbp_enemy__tendril_monst)
  (Transformation|AttachComponentToComponent (Variables|Default|GetSphere) (Variables|/Script/Engine.Character|GetMesh (Variables|Default|GetTendrilMonster_Ref)) "pelvis" "SnapToTarget" "SnapToTarget" "SnapToTarget" true))

(event EventTick
  (params (DeltaSeconds :type Float%20%28single-precision%29)))

(fn ConstructionScript)