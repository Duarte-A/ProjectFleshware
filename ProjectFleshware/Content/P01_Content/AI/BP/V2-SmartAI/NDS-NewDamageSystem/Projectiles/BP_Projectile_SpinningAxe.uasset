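; Spinning axe projectile Blueprint that adds a continuous spin to its parent projectile's behavior.
; On BeginPlay, it runs the parent logic and sets whether the box collision ignores the instigator while moving, using the IgnoreInstigator flag.
; A timeline drives the world yaw of RotationPoint, preserving pitch and roll, and calls SpinAxe again on finish to loop endlessly.
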(event Custom|SpinAxe
  (bind _rotation_point (Variables|Default|GetRotation%20Point))
  (bind _returnvalue (Transformation|GetWorldRotation _rotation_point))
  (bind _zrotation (Timeline|RotationTimeline PlayFromStart)
    (:Update
      (Transformation|SetWorldRotation (Variables|Default|GetRotation%20Point) (Math|Rotator|MakeRotator (.roll _returnvalue) (.pitch _returnvalue) _zrotation) false false))
    (:Finished
      (CallFunction|SpinAxe))))

(event EventBeginPlay
  (|CallParentFunction)
  (Collision|IgnoreActorwhenMoving (Variables|Default|GetBoxCollision) (Game|GetInstigator) (Variables|Default|GetIgnoreInstigator))
  (CallFunction|SpinAxe))

(event Collision|EventActorBeginOverlap
  (params (OtherActor :type Actor%20Object%20Reference)))

(event EventTick
  (params (DeltaSeconds :type Float%20%28single-precision%29)))

(fn ConstructionScript
  (|CallParentFunction))